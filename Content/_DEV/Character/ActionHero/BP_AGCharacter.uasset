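; Action hero character with camera-relative movement, strafing, directional dodge, sword attack and gun fire.
; Montages drive actions, with state flags gating sword attacks during other actions or falls, while the gun's IsDoingAction check always returns false.
; EquipWeapon swaps sword and gun between hand and body sockets, auto-unequipping after a retriggerable delay.
; Another character found at BeginPlay supplies the focus and an angle-limited aim rotation.
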(event Input|EnhancedActionEvents|EnhancedInputActionIA_Looks
  (params (ActionValue :type Vector%202D%20Structure) (ElapsedSeconds :type Float%20%28double-precision%29) (TriggeredSeconds :type Float%20%28double-precision%29) (InputAction :type Input%20Action%20Object%20Reference :default "/Game/_DEV/Input/IA/IA_Looks.IA_Looks"))
  (Pawn|Input|AddControllerYawInput (.x ActionValue))
  (Pawn|Input|AddControllerPitchInput (.y ActionValue)))

(event Input|EnhancedActionEvents|EnhancedInputActionIA_Moves
  (params (ActionValue :type Vector%202D%20Structure) (ElapsedSeconds :type Float%20%28double-precision%29) (TriggeredSeconds :type Float%20%28double-precision%29) (InputAction :type Input%20Action%20Object%20Reference :default "/Game/_DEV/Input/IA/IA_Moves.IA_Moves"))
  (bind _returnvalue (Pawn|GetControlRotation :!class /Script/Engine.Pawn))
  (bind _returnvalue_2 (Math|Rotator|MakeRotator 0.0 0.0 (.yaw _returnvalue)))
  (if (not (Variables|Default|GetIsLanding))
    (Pawn|Input|AddMovementInput (Math|Vector|GetRightVector _returnvalue_2) (.x ActionValue) false)
    (Pawn|Input|AddMovementInput (Math|Vector|GetForwardVector _returnvalue_2) (.y ActionValue) false)))

(event Input|EnhancedActionEvents|EnhancedInputActionIA_Strafe
  (params (ActionValue :type Boolean) (ElapsedSeconds :type Float%20%28double-precision%29) (TriggeredSeconds :type Float%20%28double-precision%29) (InputAction :type Input%20Action%20Object%20Reference :default "/Game/_DEV/Input/IA/IA_Strafe.IA_Strafe"))
  (bind _charactermovement (Variables|Character|GetCharacterMovement))
  (:Started
    (Variables|/Script/Engine.CharacterMovementComponent|SetbOrientRotationToMovement _charactermovement false))
  (:Completed
    (Variables|/Script/Engine.CharacterMovementComponent|SetbOrientRotationToMovement _charactermovement true)))

(event EventBeginPlay
  (bind _outactors (Actor|GetAllActorsOfClass "BP_AGCharacter_C"))
  (for _array_element _outactors
    (if (!= _array_element self)
      (Variables|Default|SetTargetCharacter _array_element))))

(event Collision|EventActorBeginOverlap
  (params (OtherActor :type Actor%20Object%20Reference)))

(event EventTick
  (params (DeltaSeconds :type Float%20%28single-precision%29)))

(event EventOnLanded
  (params (Hit :type Hit%20Result%20Structure%20%28by%20ref%29))
  (Variables|Default|SetIsLanding true)
  (Utilities|FlowControl|Delay 0.2)
  (Variables|Default|SetIsLanding false))

(event Input|EnhancedActionEvents|EnhancedInputActionIA_Dodge
  (params (ActionValue :type Boolean) (ElapsedSeconds :type Float%20%28double-precision%29) (TriggeredSeconds :type Float%20%28double-precision%29) (InputAction :type Input%20Action%20Object%20Reference :default "/Game/_DEV/Input/IA/IA_Dodge.IA_Dodge"))
  (bind _returnvalue (Pawn|GetControlRotation :!class /Script/Engine.Pawn))
  (bind _returnvalue_2 (Input|EnhancedActionValues|GetIA_Moves))
  (bind _returnvalue_3 (Math|Rotator|MakeRotator 0.0 0.0 (.yaw _returnvalue)))
  (bind _returnvalue_4 (Math|Conversions|ToVector(Vector2D) _returnvalue_2))
  (bind (_x _y) (Math|Vector|BreakVector _returnvalue_4))
  (if (not (Variables|Default|GetIsDodging))
    (if (not (Class|KismetMathLibrary|IsNearlyZero2D _returnvalue_2 0.0001))
      (Variables|Default|SetIsDodging true)
      (CallFunction|EquipWeapon "NewEnumerator0" true)
      (Animation|Montage|PlayMontage (Variables|Character|GetMesh) "/Game/_DEV/Character/ActionHero/Animation/AM_Evade.AM_Evade" 1.0 0.0 (Utilities|Select :Index (|(Floor((((((x+180)-45)+360)%360)/90))) (Class|KismetAnimationLibrary|CalculateDirection (+ (* _x (Math|Vector|GetRightVector _returnvalue_3)) (* _y (Math|Vector|GetForwardVector _returnvalue_3))) (Transformation|GetActorRotation))) :Option%200 "L" :Option%201 "F" :Option%202 "R" :Option%203 "B")
        (:OnBlendOut
          (Variables|Default|SetIsDodging false))))))

(event Input|EnhancedActionEvents|EnhancedInputActionIA_SwordAttack
  (params (ActionValue :type Boolean) (ElapsedSeconds :type Float%20%28double-precision%29) (TriggeredSeconds :type Float%20%28double-precision%29) (InputAction :type Input%20Action%20Object%20Reference :default "/Game/_DEV/Input/IA/IA_SwordAttack.IA_SwordAttack"))
  (:Started
    (if (not (CallFunction|CanAction))
      (Utilities|FlowControl|Sequence
        (:then_0
          (Variables|Default|SetIsSwordAttacking true)
          (bind _notifyname (Animation|Montage|PlayMontage (Variables|Character|GetMesh) "/Game/_DEV/Character/ActionHero/Animation/AM_Sword_Attack.AM_Sword_Attack")
            (:then
              (CallFunction|EquipWeapon "NewEnumerator2" false)
              (CallFunction|CancelAutoUnequip))
            (:OnCompleted
              (CallFunction|AutoUnequip))
            (:OnNotifyBegin
              (if (== _notifyname "ReleaseAttack")
                (Variables|Default|SetIsSwordAttacking false)))))
        (:then_1
          (CallFunction|MeleeHit "0, 0, 0" 0.0))))))

(event Input|EnhancedActionEvents|EnhancedInputActionIA_Fire
  (params (ActionValue :type Boolean) (ElapsedSeconds :type Float%20%28double-precision%29) (TriggeredSeconds :type Float%20%28double-precision%29) (InputAction :type Input%20Action%20Object%20Reference :default "/Game/_DEV/Input/IA/IA_Fire.IA_Fire"))
  (if (not (CallFunction|IsDoingAction))
    (Variables|Default|SetIsGunFiring true)
    (bind _notifyname (Animation|Montage|PlayMontage (Variables|Character|GetMesh) "/Game/_DEV/Character/ActionHero/Animation/AM_Gun_Fire.AM_Gun_Fire")
      (:then
        (CallFunction|EquipWeapon "NewEnumerator1" false)
        (CallFunction|CancelAutoUnequip))
      (:OnCompleted
        (CallFunction|AutoUnequip))
      (:OnNotifyBegin
        (if (== _notifyname "ReleaseAttack")
          (Variables|Default|SetIsGunFiring false))))))

(event Custom|UnequipGun
  (params (Instant :type Boolean))
  (if (Utilities|Enum|Equal(Enum) (Variables|Default|GetEquippedWeapon) "NewEnumerator1")
    (if Instant
      (Variables|Default|SetEquippedWeapon "NewEnumerator0")
      (Transformation|AttachComponentToComponent (Variables|Default|GetHolsterGun) (Variables|Character|GetMesh) "HolsterSocket" "SnapToTarget" "SnapToTarget" "KeepRelative" true)
      (else
        (bind _notifyname (Animation|Montage|PlayMontage (Variables|Character|GetMesh) "/Game/_DEV/Character/ActionHero/Animation/AM_Gun_Unequip.AM_Gun_Unequip")
          (:OnNotifyBegin
            (if (== _notifyname "WeaponDetach")
              (Transformation|AttachComponentToComponent (Variables|Default|GetHolsterGun) (Variables|Character|GetMesh) "HolsterSocket" "SnapToTarget" "SnapToTarget" "KeepRelative" true)
              (Components|MoveComponentTo (Variables|Default|GetHolsterGun) "0, 0, 0" "0, 0, 0" false false 0.3 false))))))))

(event Custom|UnequipSword
  (params (Instant :type Boolean))
  (if (Utilities|Enum|Equal(Enum) (Variables|Default|GetEquippedWeapon) "NewEnumerator2")
    (if Instant
      (Variables|Default|SetEquippedWeapon "NewEnumerator0")
      (Transformation|AttachComponentToComponent (Variables|Default|GetScabbardSword) (Variables|Character|GetMesh) "ScabbardSocket" "SnapToTarget" "SnapToTarget" "KeepRelative" true)
      (else
        (bind _notifyname (Animation|Montage|PlayMontage (Variables|Character|GetMesh) "/Game/_DEV/Character/ActionHero/Animation/AM_Sword_Unequip.AM_Sword_Unequip")
          (:OnNotifyBegin
            (if (== _notifyname "WeaponDetach")
              (Transformation|AttachComponentToComponent (Variables|Default|GetScabbardSword) (Variables|Character|GetMesh) "ScabbardSocket" "SnapToTarget" "SnapToTarget" "KeepRelative" true)
              (Components|MoveComponentTo (Variables|Default|GetScabbardSword) "0, 0, 0" "0, 0, 0" false false 0.3 false))))))))

(event Custom|AutoUnequip
  (Variables|Default|SetCanAutoUnequip true)
  (Utilities|FlowControl|RetriggerableDelay 1.0)
  (if (Variables|Default|GetCanAutoUnequip)
    (CallFunction|EquipWeapon "NewEnumerator0" false)))

(fn ConstructionScript)

(fn GetAimRotation
  (bind _returnvalue (Transformation|GetActorTransform))
  (bind _targetcharacter (Variables|Default|GetTargetCharacter))
  (bind _returnvalue_2 (Transformation|GetActorLocation _targetcharacter))
  (bind _returnvalue_3 (Math|Rotator|FindRelativeLookatRotation _returnvalue _returnvalue_2))
  (bind (_roll _pitch _yaw) (Math|Rotator|BreakRotator _returnvalue_3))
  (Utilities|IsValid (Variables|Default|GetTargetCharacter)
    (:Is%20Valid
      (if (and (Math|Float|InRange(Float) _pitch -45.0 45.0) (Math|Float|InRange(Float) _yaw -45.0 45.0))
        (return _returnvalue_3)
        (else
          (return "0, 0, 0"))))))

(fn GetFocusCharacter
  (return (Variables|Default|GetTargetCharacter)))

(fn EquipWeapon
  (params (DesiredWeapon :type WeaponType%20Enum :default "NewEnumerator0") (Instant :type Boolean))
  (if (Utilities|Enum|NotEqual(Enum) DesiredWeapon (Variables|Default|GetEquippedWeapon))
    (switch Utilities|FlowControl|Switch|SwitchonWeaponType DesiredWeapon
      (:NewEnumerator0
        (CallFunction|UnequipSword Instant)
        (CallFunction|UnequipGun Instant))
      (:NewEnumerator1
        (CallFunction|UnequipSword true)
        (Variables|Default|SetEquippedWeapon "NewEnumerator1")
        (Transformation|AttachComponentToComponent (Variables|Default|GetHolsterGun) (Variables|Character|GetMesh) "GunSocket" "KeepRelative" "KeepRelative" "KeepRelative" true))
      (:NewEnumerator2
        (CallFunction|UnequipGun true)
        (Variables|Default|SetEquippedWeapon "NewEnumerator2")
        (Transformation|AttachComponentToComponent (Variables|Default|GetScabbardSword) (Variables|Character|GetMesh) "SwordSocket" "KeepRelative" "KeepRelative" "KeepRelative" true)))))

(fn CanAction
  (return (Math|Boolean|ORBoolean (Variables|Default|GetIsSwordAttacking) (Variables|Default|GetIsDodging) (Variables|Default|GetIsLanding) (AI|Components|NavMovement|IsFalling (Variables|Character|GetCharacterMovement)) (Variables|Default|GetIsGunFiring))))

(fn CancelAutoUnequip
  (Variables|Default|SetCanAutoUnequip false))

(fn IsDoingAction
  (return false))